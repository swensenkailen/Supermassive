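; Milky Way level Blueprint actor that plays randomized MetaSound music and pulses a black hole in time with it.
; BeginPlay adds an audio component, randomizes mix, filter and BPM, then watches the MetaSound "Envelope" output.
; Tick adds the scaled envelope level to the black hole's default size.
; RandomizeParameters adds a second audio component, which receives the sine, square and saw levels instead of the main one.
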(event Custom|SetEnvelope
  (params (OutputName :type Name) (Output :type Meta%20Sound%20Output%20Structure%20%28by%20ref%29))
  (bind _returnvalue (Class|MetasoundOutputBlueprintAccess|GetFloat Output))
  (bind _output_get (Variables|Default|SetEnvelopeLevel _returnvalue)))

(event EventBeginPlay
  (Variables|Default|SetBPM (Math|Random|RandomIntegerinRange 120 140))
  ;[1 1 1] Start Music
  (bind _returnvalue (AddComponent|AddAudioComponent false))
  (bind _output_get (Variables|Default|SetAudio%20Component _returnvalue))
  (CallFunction|RandomizeParameters)
  ;[1 1 1] Set Random BPM to start
  (Audio|Parameter|SetFloatParameter _output_get "BPM" (Math|Conversions|ToFloat(Integer) (Variables|Default|GetBPM)) :!class /Script/AudioExtensions.AudioParameterControllerInterface)
  (Development|PrintString (Utilities|String|ToString(Integer) (Variables|Default|GetBPM)))
  ;[1 1 1] Receive MS Music envelope
  (MetaSoundOutput|WatchOutput (WorldSubsystems|GetMetaSoundOutputSubsystem) (Variables|Default|GetAudio%20Component) "Envelope" (delegate Custom|SetEnvelope) "None" "None" :!class /Script/MetasoundEngine.MetaSoundOutputSubsystem))

(event Collision|EventActorBeginOverlap
  (params (OtherActor :type Actor%20Object%20Reference)))

(event EventTick
  (params (DeltaSeconds :type Float%20%28single-precision%29))
  (bind _envelopelevel (Variables|Default|GetEnvelopeLevel))
  (bind _returnvalue (* _envelopelevel 0.4))
  ;[1 1 1] Pulsing black hole
  (Transformation|SetWorldScale3D (Variables|Default|GetBlackHole) (+ (Variables|Default|GetBlackHoleDefaultSize) (Math|Vector|MakeVector _returnvalue _returnvalue _returnvalue))))

(event EventDestroyed
  (Class|AudioParameterControllerInterface|SetTriggerParameter (Variables|Default|GetAudio%20Component) "None"))

(fn ConstructionScript)

(fn RandomizeParameters
  (Audio|Parameter|SetFloatParameter (Variables|Default|GetAudio%20Component) "KickLevel" (Math|Random|RandomFloatinRange 0.5 1.0) :!class /Script/AudioExtensions.AudioParameterControllerInterface)
  (Audio|Parameter|SetFloatParameter (Variables|Default|GetAudio%20Component) "SnareLevel" (Math|Random|RandomFloatinRange 0.6 1.0) :!class /Script/AudioExtensions.AudioParameterControllerInterface)
  (Audio|Parameter|SetFloatParameter (Variables|Default|GetAudio%20Component) "SynthLevel" (Math|Random|RandomFloatinRange 0.1 1.0) :!class /Script/AudioExtensions.AudioParameterControllerInterface)
  (Audio|Parameter|SetFloatParameter (Variables|Default|GetAudio%20Component) "LowPassLevel" (Math|Random|RandomFloatinRange 0.0 1.5) :!class /Script/AudioExtensions.AudioParameterControllerInterface)
  (Audio|Parameter|SetFloatParameter (Variables|Default|GetAudio%20Component) "LowPassFrequency" (Math|Random|RandomFloatinRange 5e+02 1.6e+04) :!class /Script/AudioExtensions.AudioParameterControllerInterface)
  (bind _returnvalue (AddComponent|AddAudioComponent false))
  (Audio|Parameter|SetFloatParameter _returnvalue "SineLevel" (Math|Random|RandomFloatinRange 0.1 1.0) :!class /Script/AudioExtensions.AudioParameterControllerInterface)
  (Audio|Parameter|SetFloatParameter _returnvalue "SquareLevel" (Math|Random|RandomFloatinRange 0.1 0.3) :!class /Script/AudioExtensions.AudioParameterControllerInterface)
  (Audio|Parameter|SetFloatParameter _returnvalue "SawLevel" (Math|Random|RandomFloatinRange 0.1 0.3) :!class /Script/AudioExtensions.AudioParameterControllerInterface))