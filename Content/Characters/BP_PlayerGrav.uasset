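; BP_PlayerGrav is a player-controlled physics sphere that is pulled toward other BP_PlayerGrav actors by simulated Newtonian gravity.
; Each Tick sums inverse-square attraction over all instances, itself included, without a gravitational constant.
; It prints that sum, then applies it divided by Mass as a velocity-change impulse, unscaled by delta time.
; MoveForward and MoveRight axes add impulses along the aim rotation.
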(event EventBeginPlay)

(event Collision|EventActorBeginOverlap
  (params (OtherActor :type Actor%20Object%20Reference)))

(event EventTick
  (params (DeltaSeconds :type Float%20%28single-precision%29))
  (bind _returnvalue (Transformation|GetActorLocation))
  (Variables|Default|SetImpulses "0, 0, 0")
  (bind _outactors (Actor|GetAllActorsOfClass "BP_PlayerGrav_C"))
  (for _array_element _outactors
    ;[1 1 1] Apply Newtons Universal Law of Gravitation
    (Variables|Default|SetImpulses (+ (Variables|Default|GetImpulses) (* (/ (* (Variables|Default|GetMass) (Variables|BP_PlayerGrav_C|GetMass _array_element)) (Class|KismetMathLibrary|VectorDistanceSquared _returnvalue (Transformation|GetActorLocation _array_element))) (Math|Vector|GetUnitDirection(Vector) _returnvalue (Transformation|GetActorLocation _array_element))))))
  (Development|PrintString (Utilities|String|ToString(Vector) (Variables|Default|GetImpulses)))
  (Physics|AddImpulse (Variables|Default|GetSphere) (/ (Variables|Default|GetImpulses) (Variables|Default|GetMass)) "None" true))

(event Input|AxisEvents|InputAxisMoveForward
  (params (AxisValue :type Float%20%28single-precision%29))
  (Physics|AddImpulse (Variables|Default|GetSphere) (* (Math|Vector|GetForwardVector (Pawn|GetBaseAimRotation)) (* AxisValue 1e+02)) "None" false))

(event Input|AxisEvents|InputAxisMoveRight
  (params (AxisValue :type Float%20%28single-precision%29))
  (Physics|AddImpulse (Variables|Default|GetSphere) (* (Math|Vector|GetRightVector (Pawn|GetBaseAimRotation)) (* AxisValue 1e+02)) "None" false))

(fn ConstructionScript)