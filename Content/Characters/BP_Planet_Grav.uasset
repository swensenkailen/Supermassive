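; BP_Planet_Grav is a planet actor that attracts and is attracted by every other BP_Planet_Grav through Newtonian gravity.
; BeginPlay applies its Mass variable as the static mesh's mass scale.
; Each Tick sums inverse-square pulls over all instances, itself included, with no gravitational constant.
; It applies that sum divided by Mass as a velocity-change impulse, without delta-time scaling.
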(event EventBeginPlay
  (Class|PrimitiveComponent|SetMassScale (Variables|Debug|GetStaticMeshComponent) "None" (Variables|Default|GetMass)))

(event Collision|EventActorBeginOverlap
  (params (OtherActor :type Actor%20Object%20Reference)))

(event EventTick
  (params (DeltaSeconds :type Float%20%28single-precision%29))
  (bind _returnvalue (Transformation|GetActorLocation))
  (Variables|Default|SetImpluses "0, 0, 0")
  (bind _outactors (Actor|GetAllActorsOfClass "BP_Planet_Grav_C"))
  (for _array_element _outactors
    ;[1 1 1] Apply Newtons Universal Law of Gravitation
    (Variables|Default|SetImpluses (+ (Variables|Default|GetImpluses) (* (/ (* (Variables|Default|GetMass) (Variables|BP_Planet_Grav_C|GetMass _array_element)) (Class|KismetMathLibrary|VectorDistanceSquared _returnvalue (Transformation|GetActorLocation _array_element))) (Math|Vector|GetUnitDirection(Vector) _returnvalue (Transformation|GetActorLocation _array_element))))))
  (Physics|AddImpulse (Variables|Debug|GetStaticMeshComponent) (/ (Variables|Default|GetImpluses) (Variables|Default|GetMass)) "None" true))

(fn ConstructionScript)