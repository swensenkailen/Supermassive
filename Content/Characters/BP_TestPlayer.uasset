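; BP_TestPlayer is a test player pawn that moves by pushing its Sphere component with physics impulses.
; The MoveForward and MoveRight axis inputs scale the forward and right vectors of the base aim rotation, so movement follows the aim direction.
; Each axis event applies a mass-dependent impulse without delta-time scaling.
; BeginPlay, Tick, overlap and construction logic are empty.
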(event EventBeginPlay)

(event Collision|EventActorBeginOverlap
  (params (OtherActor :type Actor%20Object%20Reference)))

(event EventTick
  (params (DeltaSeconds :type Float%20%28single-precision%29)))

(event Input|AxisEvents|InputAxisMoveForward
  (params (AxisValue :type Float%20%28single-precision%29))
  (Physics|AddImpulse (Variables|Default|GetSphere) (* (Math|Vector|GetForwardVector (Pawn|GetBaseAimRotation)) (* AxisValue 1e+02)) "None" false))

(event Input|AxisEvents|InputAxisMoveRight
  (params (AxisValue :type Float%20%28single-precision%29))
  (Physics|AddImpulse (Variables|Default|GetSphere) (* (Math|Vector|GetRightVector (Pawn|GetBaseAimRotation)) (* AxisValue 1e+02)) "None" false))

(fn ConstructionScript)